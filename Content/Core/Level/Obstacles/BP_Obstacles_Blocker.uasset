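; BP_Obstacles_Blocker is a runner obstacle that kills the player unless they are sliding when they touch it.
; Its Box overlap casts the other actor to BP_CryptoRunnerCharacter and checks IsSliding.
; A non-sliding player triggers PlayerDeath, and the game pauses after a short delay.
; An unconnected copy of this logic never runs, and the actor-level overlap event is empty.
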(event `self.ReceiveActorBeginOverlap`
  (params (OtherActor :type "Actor Object Reference")))

(event `self.Box.OnComponentBeginOverlap`
  (params (OverlappedComponent :type "PrimitiveComponent Object Reference") (OtherActor :type "Actor Object Reference") (OtherComp :type "PrimitiveComponent Object Reference") (OtherBodyIndex :type Integer) (bFromSweep :type Boolean) (SweepResult :type "HitResult Structure (by ref)"))
  (bind _asbp_crypto_runner_character (cast `/Game/Core/Blueprints/BP_CryptoRunnerCharacter` OtherActor))
  (if (not (`/Game/Core/Blueprints/BP_CryptoRunnerCharacter.isSliding?` _asbp_crypto_runner_character))
    (`/Game/Core/Blueprints/BP_CryptoRunnerCharacter.PlayerDeath` _asbp_crypto_runner_character)
    (`KismetSystemLibrary.Delay` 1.0)
    (`GameplayStatics.SetGamePaused` true)))

(fn `UserConstructionScript`
  (`parent.UserConstructionScript`))