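; Endless-runner floor tile that, when the runner overlaps its box, calls ExtendFloor on the game mode and slightly raises walk speed up to a cap.
; The construction script builds lane spawn points, scatters random obstacles, coins and an occasional power-up as child actors, and randomizes building heights and materials.
; GetAttachedPoint exposes an attachment transform, while ClearFloor destroys coins and power-ups and clears spawn-point arrays.
; Obstacle pooling code exists but is disconnected.
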(event `self.Box.OnComponentBeginOverlap`
  (params (OverlappedComponent :type "PrimitiveComponent Object Reference") (OtherActor :type "Actor Object Reference") (OtherComp :type "PrimitiveComponent Object Reference") (OtherBodyIndex :type Integer) (bFromSweep :type Boolean) (SweepResult :type "HitResult Structure (by ref)"))
  (cast `/Game/Core/Blueprints/BP_CryptoRunnerCharacter` OtherActor)
  (bind _asbp_crypto_runner_game_mode (cast `/Game/Core/Blueprints/BP_CryptoRunnerGameMode` (`GameplayStatics.GetGameMode`)))
  (`/Game/Core/Blueprints/BP_CryptoRunnerGameMode.ExtendFloor` _asbp_crypto_runner_game_mode)
  (bind _asbp_crypto_runner_character (cast `/Game/Core/Blueprints/BP_CryptoRunnerCharacter` (`GameplayStatics.GetPlayerCharacter` 0)))
  (bind _charactermovement (`Character.CharacterMovement` _asbp_crypto_runner_character))
  (set `CharacterMovementComponent.MaxWalkSpeed` (`KismetMathLibrary.FClamp` (* (`CharacterMovementComponent.MaxWalkSpeed` _charactermovement) 1.008) 750.0 2500.0) _charactermovement))

(fn `ClearFloor`
  (locals (TempArray :type "Array of Actor Object Reference"))
  (for _array_element (`self.GetAllChildActors` true)
    (`|ExecutionSequence`
      (:`then_0`
        (bind _asbp_coin (cast `/Game/Core/Level/BP_Coin` _array_element))
        (`KismetArrayLibrary.Array_Add` (`local.TempArray`) _asbp_coin))
      (:`then_1`
        (bind _asbp_powerup (cast `/Game/Core/Level/BP_Powerup` _array_element))
        (`KismetArrayLibrary.Array_Add` (`local.TempArray`) _asbp_powerup))))
  (for _array_element_2 (`local.TempArray`)
    (`self.K2_DestroyActor` _array_element_2))
  (`KismetArrayLibrary.Array_Clear` (`self.SpawnPoints`))
  (`KismetArrayLibrary.Array_Clear` (`self.SpawnPoints_Coin`))
  (`KismetArrayLibrary.Array_Clear` (`self.SpawnPoints_PowerUp`)))

(fn `CoinSpawnPoints`
  (for _array_element (`self.LanePos`)
    (for _index (range 10)
      (bind _returnvalue (`AddComponent|NODE_AddArrowComponent-1` :`RelativeTransform` (`KismetMathLibrary.MakeTransform` (`KismetMathLibrary.MakeVector` (* _index 75.0) _array_element))))
      (`ArrowComponent.SetArrowColor` _returnvalue (struct :`R` 1.0 :`G` 1.0 :`B` 1.0 :`A` 1.0))
      (`KismetArrayLibrary.Array_Add` (`self.SpawnPoints_Coin`) (`SceneComponent.K2_GetComponentToWorld` _returnvalue)))))

(fn `GetAttachedPoint`
  (returns (ReturnValue :type "Transform Structure"))
  (return (`SceneComponent.K2_GetComponentToWorld` (`self.Arrow`))))

(fn `PowerUpSpawnPoints`
  (for _array_element (`self.LanePos`)
    (for _index (range 1 2)
      (bind _returnvalue (`AddComponent|NODE_AddArrowComponent-2` :`RelativeTransform` (`KismetMathLibrary.MakeTransform` (`KismetMathLibrary.MakeVector` (* _index 250.0) _array_element))))
      (`ArrowComponent.SetArrowColor` _returnvalue (struct :`G` 0.968981 :`B` 1.0 :`A` 1.0))
      (`KismetArrayLibrary.Array_Add` (`self.SpawnPoints_PowerUp`) (`SceneComponent.K2_GetComponentToWorld` _returnvalue)))))

(fn `PrespawnObstacles`
  (for _ (range 5)
    (`|ExecutionSequence`
      (:`then_0`
        (bind _returnvalue (`AddComponent|NODE_AddChildActorComponent-6` :`RelativeTransform` (`KismetMathLibrary.MakeRelativeTransform` (`KismetMathLibrary.MakeTransform` (0.0 0.0 -1000.0)) (`self.GetTransform`))))
        (`ActorComponent.SetActive` _returnvalue false false)
        (`KismetArrayLibrary.Array_Add` (`self.Obstacles_blocker`) _returnvalue)))))

(fn `SetUpBuildings`
  (locals (Materials :type "Array of MaterialInstance Object Reference"))
  (bind _returnvalue (`KismetMathLibrary.RandomFloatInRange` -100.0 450.0))
  (bind _returnvalue_2 (`KismetMathLibrary.RandomFloatInRange` -100.0 450.0))
  (bind _returnvalue_3 (`KismetMathLibrary.RandomFloatInRange` -100.0 450.0))
  (bind _returnvalue_4 (`KismetMathLibrary.RandomFloatInRange` -100.0 450.0))
  (bind _building2 (`self.Building2`))
  (bind _building5 (`self.Building5`))
  (bind _building6 (`self.Building6`))
  (bind _building3 (`self.Building3`))
  (bind _building7 (`self.Building7`))
  (bind _building4 (`self.Building4`))
  (bind _building1 (`self.Building1`))
  (bind _building8 (`self.Building8`))
  (`|ExecutionSequence`
    (:`then_0`
      (`SceneComponent.K2_SetRelativeLocation` _building1 (`KismetMathLibrary.MakeVector` (.x (`SceneComponent.RelativeLocation` _building1)) (.y (`SceneComponent.RelativeLocation` _building1)) _returnvalue_4) false false)
      (`SceneComponent.K2_SetRelativeLocation` _building8 (`KismetMathLibrary.MakeVector` (.x (`SceneComponent.RelativeLocation` _building8)) (.y (`SceneComponent.RelativeLocation` _building8)) _returnvalue_4) false false)
      (`PrimitiveComponent.SetMaterial` (`self.Building1`) 0 (`KismetArrayLibrary.Array_Random` (`local.Materials`)))
      (`PrimitiveComponent.SetMaterial` (`self.Building8`) 0 (`KismetArrayLibrary.Array_Random` (`local.Materials`))))
    (:`then_1`
      (`SceneComponent.K2_SetRelativeLocation` _building2 (`KismetMathLibrary.MakeVector` (.x (`SceneComponent.RelativeLocation` _building2)) (.y (`SceneComponent.RelativeLocation` _building2)) _returnvalue_2) false false)
      (`SceneComponent.K2_SetRelativeLocation` _building5 (`KismetMathLibrary.MakeVector` (.x (`SceneComponent.RelativeLocation` _building5)) (.y (`SceneComponent.RelativeLocation` _building5)) _returnvalue_2) false false)
      (`PrimitiveComponent.SetMaterial` (`self.Building2`) 0 (`KismetArrayLibrary.Array_Random` (`local.Materials`)))
      (`PrimitiveComponent.SetMaterial` (`self.Building5`) 0 (`KismetArrayLibrary.Array_Random` (`local.Materials`))))
    (:`then_2`
      (`SceneComponent.K2_SetRelativeLocation` _building3 (`KismetMathLibrary.MakeVector` (.x (`SceneComponent.RelativeLocation` _building3)) (.y (`SceneComponent.RelativeLocation` _building3)) _returnvalue_3) false false)
      (`SceneComponent.K2_SetRelativeLocation` _building6 (`KismetMathLibrary.MakeVector` (.x (`SceneComponent.RelativeLocation` _building6)) (.y (`SceneComponent.RelativeLocation` _building6)) _returnvalue_3) false false)
      (`PrimitiveComponent.SetMaterial` (`self.Building3`) 0 (`KismetArrayLibrary.Array_Random` (`local.Materials`)))
      (`PrimitiveComponent.SetMaterial` (`self.Building6`) 0 (`KismetArrayLibrary.Array_Random` (`local.Materials`))))
    (:`then_3`
      (`SceneComponent.K2_SetRelativeLocation` _building4 (`KismetMathLibrary.MakeVector` (.x (`SceneComponent.RelativeLocation` _building4)) (.y (`SceneComponent.RelativeLocation` _building4)) _returnvalue) false false)
      (`SceneComponent.K2_SetRelativeLocation` _building7 (`KismetMathLibrary.MakeVector` (.x (`SceneComponent.RelativeLocation` _building7)) (.y (`SceneComponent.RelativeLocation` _building7)) _returnvalue) false false)
      (`PrimitiveComponent.SetMaterial` (`self.Building4`) 0 (`KismetArrayLibrary.Array_Random` (`local.Materials`)))
      (`PrimitiveComponent.SetMaterial` (`self.Building7`) 0 (`KismetArrayLibrary.Array_Random` (`local.Materials`))))))

(fn `SetupFloor`
  (`self.SetupSpawnPoints`)
  (`self.SpawnObastacles`)
  (`self.SetUpBuildings`)
  (`self.CoinSpawnPoints`)
  (`self.SpawnCoins`)
  (if (not (> (`KismetMathLibrary.RandomFloatInRange` 0.0 1.0) 0.1))
    (`self.PowerUpSpawnPoints`)
    (`self.SpawnPowerups`)))

(fn `SetupSpawnPoints`
  (locals (arrowCount :type Integer))
  (bind _arrowcount (`local.arrowCount`))
  (for _array_element (`self.LanePos`)
    (for _index (range 2)
      (if (> (`KismetArrayLibrary.Array_Length` (`self.Arrows`)) (`local.arrowCount`))
        (bind _returnvalue (`KismetMathLibrary.MakeTransform` (`KismetMathLibrary.MakeVector` (* _index 650.0) _array_element)))
        (`SceneComponent.K2_SetRelativeTransform` (`|GetArrayItem` (`self.Arrows`) (`local.arrowCount`)) _returnvalue false false)
        (`/Engine/EditorBlueprintResources/StandardMacros.IncrementInt` (`local.arrowCount`))
        (else
          (bind _returnvalue_2 (`AddComponent|NODE_AddArrowComponent-0` :`RelativeTransform` _returnvalue))
          (`KismetArrayLibrary.Array_Add` (`self.SpawnPoints`) (`SceneComponent.K2_GetComponentToWorld` _returnvalue_2))
          (`KismetArrayLibrary.Array_Set` (`self.Arrows`) _arrowcount _returnvalue_2 true)
          (`/Engine/EditorBlueprintResources/StandardMacros.IncrementInt` _arrowcount))))))

(fn `SpawnCoins`
  (locals (RandomSpawnPoints :type "Array of Transform Structure"))
  (bind _output_get (set `local.RandomSpawnPoints` (`self.SpawnPoints_Coin`)))
  (`KismetArrayLibrary.Array_Shuffle` _output_get)
  (for _index (range (+ (`KismetMathLibrary.RandomIntegerInRange` 5 9) 1))
    (switch `int` 0
      (:`0`
        (`AddComponent|NODE_AddChildActorComponent-2` :`RelativeTransform` (`KismetMathLibrary.MakeRelativeTransform` (`|GetArrayItem` (`local.RandomSpawnPoints`) _index) (`self.GetTransform`)))))))

(fn `SpawnObastacles`
  (locals (RandomSpawnPoints :type "Array of Transform Structure"))
  (bind _output_get (set `local.RandomSpawnPoints` (`self.SpawnPoints`)))
  (`KismetArrayLibrary.Array_Shuffle` _output_get)
  (for _index (range (+ (`KismetMathLibrary.RandomIntegerInRange` 0 2) 1))
    (switch `int` (`KismetMathLibrary.RandomIntegerInRange` 0 2)
      (:`0`
        (bind _returnvalue (`KismetMathLibrary.MakeRelativeTransform` (`|GetArrayItem` (`local.RandomSpawnPoints`) _index) (`self.GetTransform`)))
        (`AddComponent|NODE_AddChildActorComponent-0` :`RelativeTransform` _returnvalue))
      (:`1`
        (`AddComponent|NODE_AddChildActorComponent-1` :`RelativeTransform` _returnvalue))
      (:`2`
        (`AddComponent|NODE_AddChildActorComponent-4` :`RelativeTransform` _returnvalue)))))

(fn `SpawnPowerups`
  (locals (RandomSpawnPoints :type "Array of Transform Structure"))
  (bind _output_get (set `local.RandomSpawnPoints` (`self.SpawnPoints_PowerUp`)))
  (`KismetArrayLibrary.Array_Shuffle` _output_get)
  (`AddComponent|NODE_AddChildActorComponent-5` :`RelativeTransform` (`KismetMathLibrary.MakeRelativeTransform` (`|GetArrayItem` (`local.RandomSpawnPoints`)) (`self.GetTransform`))))

(fn `UserConstructionScript`
  (`self.SetupFloor`))