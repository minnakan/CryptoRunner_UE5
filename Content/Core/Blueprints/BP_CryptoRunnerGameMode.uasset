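; Game mode for an endless runner that builds the track from BP_Floor tiles and tracks the score.
; BeginPlay chains the initial tiles, each spawned at the previous one's attach point; ExtendFloor appends another and destroys the oldest once the count passes a threshold.
; Tick derives CurrentPoints from the player's forward X distance.
; Floor pooling functions exist but are disconnected, noted as broken when resetting child actors.
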(event `self.ReceiveBeginPlay`
  (for _ (range (`self.TileCount`))
    (`self.AddFloor`)))

(event `self.ReceiveTick`
  (params (DeltaSeconds :type "Float (single-precision)"))
  (bind _asbp_crypto_runner_character (cast `/Game/Core/Blueprints/BP_CryptoRunnerCharacter` (`GameplayStatics.GetPlayerCharacter` 0)))
  (bind _x (.x (`SceneComponent.K2_GetComponentLocation` (`Character.Mesh` _asbp_crypto_runner_character))))
  (set `self.CurrentPoints` (/ (`KismetMathLibrary.FTrunc` (* _x (> _x 0.0))) 100)))

(fn `AddFloor`
  (locals (TempBP_Floor :type "/Game/Core/Level/BP_Floor Object Reference"))
  (bind _returnvalue (`|SpawnActorFromClass` "/Game/Core/Level/BP_Floor.BP_Floor_C" (`self.FloorPoint`) "Undefined" "MultiplyWithRoot" null null))
  (bind _returnvalue_2 (`/Game/Core/Level/BP_Floor.GetAttachedPoint` _returnvalue))
  (set `self.FloorPoint` _returnvalue_2)
  (`KismetArrayLibrary.Array_Add` (`self.FloorTiles`) _returnvalue))

(fn `Deactivate Floor`
  (params (index :type Integer))
  (locals (TempFloor :type "/Game/Core/Level/BP_Floor Object Reference"))
  (if (`KismetArrayLibrary.Array_IsValidIndex` (`self.FloorTiles`) index)
    (bind _output_get (set `local.TempFloor` (`|GetArrayItem` (`self.FloorTiles`) index)))
    (`KismetArrayLibrary.Array_RemoveItem` (`self.FloorTiles`) _output_get)
    (`/Game/Core/Level/BP_Floor.ClearFloor` _output_get)
    (`self.SetActorHiddenInGame` _output_get true)
    (`BlueprintSetLibrary.Set_Add` (`self.OP_FloorTiles`) _output_get)
    (`ActorComponent.Deactivate` (`/Game/Core/Level/BP_Floor.DefaultSceneRoot` _output_get))
    (`SceneComponent.K2_SetWorldTransform` (`/Game/Core/Level/BP_Floor.DefaultSceneRoot` _output_get) (`KismetMathLibrary.MakeTransform` (0.0 0.0 -10000.0)) false true)
    (else
      (`KismetSystemLibrary.PrintString` "should not reach here!!"))))

(fn `ExtendFloor`
  (bind _floortiles (`self.FloorTiles`))
  (bind _output (`|GetArrayItem` _floortiles))
  (`self.AddFloor`)
  (if (> (`KismetArrayLibrary.Array_Length` (`self.FloorTiles`)) (+ (`self.TileCount`) 3))
    (`self.K2_DestroyActor` _output)
    (`KismetArrayLibrary.Array_RemoveItem` _floortiles _output)))

(fn `PoolFloors`
  (params (Count :type Integer))
  (for _ (range 1 (+ Count 1))
    (bind _returnvalue (`|SpawnActorFromClass` "/Game/Core/Level/BP_Floor.BP_Floor_C" (`KismetMathLibrary.MakeTransform` (0.0 0.0 -10000.0)) "Undefined" "MultiplyWithRoot" null null))
    (`self.SetActorHiddenInGame` _returnvalue true)
    (`ActorComponent.Deactivate` (`/Game/Core/Level/BP_Floor.DefaultSceneRoot` _returnvalue))
    (`BlueprintSetLibrary.Set_Add` (`self.OP_FloorTiles`) _returnvalue)
    (`/Game/Core/Level/BP_Floor.GetAttachedPoint` _returnvalue)))

(fn `UserConstructionScript`)