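; Player character for a three-lane endless runner that runs forward automatically and can jump, slide and switch lanes.
; A timeline lerps Y between clamped lanes, while sliding applies a downward impulse and, when moving on the ground, plays a montage and temporarily ignores Destructible collision.
; A retriggerable delay times the magnet powerup.
; PlayerDeath ragdolls the mesh, shows the game-over UI and saves any new high score from the game mode.
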(event `self.ReceiveBeginPlay`
  (bind _asplayer_controller (cast `PlayerController` (`self.GetController`)))
  (bind _returnvalue (pcsubsystem `EnhancedInputLocalPlayerSubsystem` _asplayer_controller))
  (`/Engine/EditorBlueprintResources/StandardMacros.IsValid` _returnvalue
    (:`Is Valid`
      (`EnhancedInputSubsystemInterface.AddMappingContext` _returnvalue "/Game/Core/Input/IMC_CryptoRunnerDefault.IMC_CryptoRunnerDefault" 0 (struct))
      (bind _returnvalue_2 (`|CreateWidget` "/Game/Core/UI/UI_Gameplay.UI_Gameplay_C"))
      (`UserWidget.AddToViewport` _returnvalue_2 0))))

(event `self.ReceiveTick`
  (params (DeltaSeconds :type "Float (single-precision)"))
  ;[0 0 0] Infinite Run
  (`self.AddMovementInput` (`KismetMathLibrary.GetForwardVector` (`KismetMathLibrary.MakeRotator` 0.0 0.0 (.yaw (`self.GetControlRotation`))))))

(event `EnhancedInput|/Game/Core/Input/IA_JumpCrypto`
  (params (ActionValue :type Boolean) (ElapsedSeconds :type "Float (double-precision)") (TriggeredSeconds :type "Float (double-precision)") (InputAction :type "InputAction Object Reference" :default "/Game/Core/Input/IA_JumpCrypto.IA_JumpCrypto"))
  (:`Triggered`
    (`self.Jump`)))

(event `EnhancedInput|/Game/Core/Input/IA_SlideCrypto`
  (params (ActionValue :type Boolean) (ElapsedSeconds :type "Float (double-precision)") (TriggeredSeconds :type "Float (double-precision)") (InputAction :type "InputAction Object Reference" :default "/Game/Core/Input/IA_SlideCrypto.IA_SlideCrypto"))
  (bind _charactermovement (`self.CharacterMovement`))
  (:`Triggered`
    (`CharacterMovementComponent.AddImpulse` (`self.CharacterMovement`) (0.0 0.0 -1000.0) true)
    (if (and (> (`KismetMathLibrary.VSize` (`MovementComponent.Velocity` _charactermovement)) 60.0) (not (`NavMovementComponent.IsFalling` _charactermovement)))
      (`/Engine/EditorBlueprintResources/StandardMacros.DoOnce` false :!label _label
        (:`Completed`
          (`self.DisableInput` null)
          (`PrimitiveComponent.SetCollisionResponseToChannel` (`self.CapsuleComponent`) "ECC_Destructible" "ECR_Ignore")
          (set `self.isSliding?` true)
          (`AnimInstance.Montage_Play` (`SkeletalMeshComponent.GetAnimInstance` (`self.Mesh`)) "/Game/Core/Animations/Running_Slide_Retargeted_Montage_Fixed.Running_Slide_Retargeted_Montage_Fixed" 1.5 "MontageLength" 0.0 true)
          (`KismetSystemLibrary.Delay` 0.7)
          (`PrimitiveComponent.SetCollisionResponseToChannel` (`self.CapsuleComponent`) "ECC_Destructible" "ECR_Block")
          (`self.EnableInput` null)
          (set `self.isSliding?` false)
          (goto _label :!via `Reset`))))))

(event `ChangeLanes`
  (params (ChangeLane :type Integer))
  (set `self.targetLane` (`KismetMathLibrary.Clamp` (+ ChangeLane (`self.currentLane`)) 0 2))
  (set `self.CurrentPosY` (.y (`self.K2_GetActorLocation`)))
  (bind (_direction _lanechange) (`Timeline|Timeline` :!via `PlayFromStart`)
    (:`Update`
      (`self.K2_SetActorLocation` (`KismetMathLibrary.MakeVector` (.x (`self.K2_GetActorLocation`)) (`KismetMathLibrary.Lerp` (`self.CurrentPosY`) (`|GetArrayItem` (`self.LanePos`) (`self.targetLane`)) _lanechange) (.z (`self.K2_GetActorLocation`)))))
    (:`Finished`
      (set `self.currentLane` (`self.targetLane`)))))

(event `EnhancedInput|/Game/Core/Input/IA_LeftCrypto`
  (params (ActionValue :type Boolean) (ElapsedSeconds :type "Float (double-precision)") (TriggeredSeconds :type "Float (double-precision)") (InputAction :type "InputAction Object Reference" :default "/Game/Core/Input/IA_LeftCrypto.IA_LeftCrypto"))
  (:`Started`
    (`self.ChangeLanes` -1)))

(event `EnhancedInput|/Game/Core/Input/IA_RightCrypto`
  (params (ActionValue :type Boolean) (ElapsedSeconds :type "Float (double-precision)") (TriggeredSeconds :type "Float (double-precision)") (InputAction :type "InputAction Object Reference" :default "/Game/Core/Input/IA_RightCrypto.IA_RightCrypto"))
  (:`Started`
    (`self.ChangeLanes` 1)))

(event `ActivatePowerup`
  (set `self.isMagnetActive?` true)
  (`KismetSystemLibrary.RetriggerableDelay` 5.0)
  (set `self.isMagnetActive?` false))

(fn `PlayerDeath`
  (`CharacterMovementComponent.DisableMovement` (`self.CharacterMovement`))
  (`self.DisableInput` null)
  (`PrimitiveComponent.SetSimulatePhysics` (`self.Mesh`) true)
  (`WidgetLayoutLibrary.RemoveAllWidgets`)
  (bind _returnvalue (`|CreateWidget` "/Game/Core/UI/UI_GameOver.UI_GameOver_C"))
  (`UserWidget.AddToViewport` _returnvalue 0)
  (set `PlayerController.bShowMouseCursor` true (`GameplayStatics.GetPlayerController` 0))
  (bind _asbp_crypto_runner_game_mode (cast `/Game/Core/Blueprints/BP_CryptoRunnerGameMode` (`GameplayStatics.GetGameMode`)))
  (bind _returnvalue_2 (`GameplayStatics.DoesSaveGameExist` "HighScore"))
  (if _returnvalue_2
    (bind _returnvalue_3 (`GameplayStatics.LoadGameFromSlot` "HighScore"))
    (bind _output_get (set `self.Saver` _returnvalue_3))
    (bind _asbp_crypto_save_game (cast `/Game/Core/Blueprints/BP_CryptoSaveGame` _output_get))
    (bind _currentpoints (`/Game/Core/Blueprints/BP_CryptoRunnerGameMode.CurrentPoints` _asbp_crypto_runner_game_mode))
    (if (> _currentpoints (`/Game/Core/Blueprints/BP_CryptoSaveGame.HighScore` _asbp_crypto_save_game))
      (set `/Game/Core/Blueprints/BP_CryptoSaveGame.HighScore` _currentpoints _asbp_crypto_save_game)
      (`GameplayStatics.SaveGameToSlot` (`self.Saver`) "HighScore"))
    (else
      (bind _returnvalue_4 (`GameplayStatics.CreateSaveGameObject` "/Game/Core/Blueprints/BP_CryptoSaveGame.BP_CryptoSaveGame_C"))
      (bind _output_get_2 (set `self.Saver` _returnvalue_4))
      (bind _asbp_crypto_save_game_2 (cast `/Game/Core/Blueprints/BP_CryptoSaveGame` _output_get_2))
      (set `/Game/Core/Blueprints/BP_CryptoSaveGame.HighScore` _currentpoints _asbp_crypto_save_game_2)
      (`GameplayStatics.SaveGameToSlot` (`self.Saver`) "HighScore"))))

(fn `UserConstructionScript`)